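; BP_GeneralButton is a VR puzzle button that toggles between pressed and unpressed when a VRPawn overlaps its collision.
; Press and Unpress run the AnimacionBoton macro to slide the button mesh, then update the state and fire OnPressAction or OnUnPressAction, both placeholder prints here.
; BeginPlay caches the BP_EventManager and automatically presses the button after a short delay.
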(event `self.ReceiveBeginPlay`
  (bind _returnvalue (`GameplayStatics.GetActorOfClass` "/Game/Dynamic/Blueprints/BP_EventManager.BP_EventManager_C"))
  (set `self.EventManager` _returnvalue)
  (`KismetSystemLibrary.Delay` 5.0)
  (`self.Press`))

(event `/Game/Dynamic/Blueprints/Interfaces/BPI_Button.Unpress`
  (if (`self.isButtonPressed`)
    (`self.AnimacionBoton`
      (:`Completed`
        (set `self.isButtonPressed` false)
        (`self.OnUnPressAction`)))))

(event `/Game/Dynamic/Blueprints/Interfaces/BPI_Button.Press`
  (if (not (`self.isButtonPressed`))
    (`self.AnimacionBoton`
      (:`Completed`
        (set `self.isButtonPressed` true)
        (`self.OnPressAction`)))))

(event `self.ButtonCollision.OnComponentBeginOverlap`
  (params (OverlappedComponent :type "PrimitiveComponent Object Reference") (OtherActor :type "Actor Object Reference") (OtherComp :type "PrimitiveComponent Object Reference") (OtherBodyIndex :type Integer) (bFromSweep :type Boolean) (SweepResult :type "HitResult Structure (by ref)"))
  (cast `/Game/Dynamic/Blueprints/VR_Template/VRPawn` OtherActor)
  (if (`self.isButtonPressed`)
    (`self.Unpress`)
    (else
      (`self.Press`))))

(event `/Game/Dynamic/Blueprints/Interfaces/BPI_Button.OnPressAction`
  (`KismetSystemLibrary.PrintString` "ON PRESS ACTION WIP"))

(event `/Game/Dynamic/Blueprints/Interfaces/BPI_Button.OnUnPressAction`
  (`KismetSystemLibrary.PrintString` "ON UNPRESS ACTION WIP"))

(fn `isPressed`
  (returns (isPressed :type Boolean))
  (return (`self.isButtonPressed`)))

(fn `UserConstructionScript`)