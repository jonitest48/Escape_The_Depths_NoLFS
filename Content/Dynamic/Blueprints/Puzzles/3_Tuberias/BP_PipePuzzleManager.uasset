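; Manager for the pipe puzzle that decides when every pipe actor in its PipePuzzleActors array is fixed.
; On BeginPlay it binds CheckAllFixed to the ED Check All Fixed dispatcher, then prints the pipe names after a short delay for debugging.
; Each check stops at the first unfixed pipe, or, if all are fixed, calls CompletePuzzle on BP_EndGamePad with its PuzzleNumber.
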(event `self.ReceiveBeginPlay`
  (add `self.ED_CheckAllFixed` (delegate `CheckAllFixed`))
  (`KismetSystemLibrary.Delay` 1.0)
  (for _array_element (`self.PipePuzzleActors`)
    (`KismetSystemLibrary.PrintString` (`KismetSystemLibrary.GetDisplayName` _array_element))))

(event `CheckAllFixed`
  ;[1 1 1] Check all PipePuzzle Actors are fixed
  (if (`KismetArrayLibrary.Array_IsNotEmpty` (`self.PipePuzzleActors`))
    (set `self.isSolved` true)
    (for _array_element (`self.PipePuzzleActors`)
      (if (not (`/Game/Dynamic/Blueprints/Puzzles/3_Tuberias/BP_PipePuzzleActor.isFixed` _array_element))
        (set `self.isSolved` false)
        (`KismetSystemLibrary.PrintString` (`KismetStringLibrary.Concat_StrStr` (`KismetSystemLibrary.GetDisplayName` _array_element) "No está solucionado todavia"))
        (break)))
    (if (`self.isSolved`)
      (`KismetSystemLibrary.PrintString` "Resuelto")
      (bind _returnvalue (`GameplayStatics.GetActorOfClass` "/Game/Dynamic/Blueprints/Puzzles/5_EndGame/BP_EndGamePad.BP_EndGamePad_C"))
      (`/Game/Dynamic/Blueprints/Puzzles/5_EndGame/BP_EndGamePad.CompletePuzzle` _returnvalue (`self.PuzzleNumber`))
      (else
        (`KismetSystemLibrary.PrintString` "Sin Resolver")))))

(fn `UserConstructionScript`)