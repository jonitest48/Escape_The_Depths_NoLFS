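; BP_Pipe is a grabbable, physics-simulated pipe piece for the pipe puzzle that raises a sound alert on hard impacts.
; The construction script picks a straight, curved, intersection or broken mesh from PipeType and sets the grab type.
; On hit, velocity times mass is tested against a threshold, then SoundAlertAtLocation receives the level's BP_EventManager.
; A Gate blocks repeat alerts for half the sound's duration.
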(event `self.ReceiveBeginPlay`
  (bind _returnvalue (`GameplayStatics.GetActorOfClass` "/Game/Dynamic/Blueprints/BP_EventManager.BP_EventManager_C"))
  (set `self.EventManager` _returnvalue))

(event `self.Pipe.OnComponentHit`
  (params (HitComponent :type "PrimitiveComponent Object Reference") (OtherActor :type "Actor Object Reference") (OtherComp :type "PrimitiveComponent Object Reference") (NormalImpulse :type "Vector Structure") (Hit :type "HitResult Structure (by ref)"))
  (bind _sound (`self.Sound`))
  (bind _returnvalue (* (`KismetMathLibrary.VSize` (`self.GetVelocity` self)) (`PrimitiveComponent.GetMass` HitComponent)))
  (if (`SceneComponent.IsSimulatingPhysics` HitComponent "None")
    (if (>= _returnvalue 1000.0)
      (`/Engine/EditorBlueprintResources/StandardMacros.Gate` false :!label _label
        (:`Exit`
          (`|ExecutionSequence`
            (:`then_0`
              (`KismetSystemLibrary.PrintString` (`KismetStringLibrary.Concat_StrStr` "FORCE OF IMPACT: " (`KismetStringLibrary.Conv_DoubleToString` _returnvalue)) true true (struct :`G` 0.66 :`B` 1.0 :`A` 1.0) 0.5)
              (goto _label :!via `Close`))
            (:`then_1`
              (`/Game/Dynamic/Blueprints/MonsterEvents/3_Silence/BP_SilenceEventFunctions.SoundAlertAtLocation` _sound Hit_Location (`self.EventManager`))
              (`KismetSystemLibrary.Delay` (/ (`SoundBase.Duration` _sound) 2.0))
              (goto _label :!via `Open`))))))))

(fn `UserConstructionScript`
  (bind _pipe (`self.Pipe`))
  (switch `/Game/Dynamic/Blueprints/Puzzles/3_Tuberias/E_PipeTypes` (`self.PipeType`)
    (:`NewEnumerator0`
      (`StaticMeshComponent.SetStaticMesh` _pipe "/Game/Static/Meshes/Tuberia_Recta.Tuberia_Recta"))
    (:`NewEnumerator1`
      (`StaticMeshComponent.SetStaticMesh` _pipe "/Game/Static/Meshes/Tuberia_Curva.Tuberia_Curva"))
    (:`NewEnumerator2`
      (`StaticMeshComponent.SetStaticMesh` _pipe "/Game/Static/Meshes/Tuberia_Intersec.Tuberia_Intersec"))
    (:`NewEnumerator3`
      (`StaticMeshComponent.SetStaticMesh` _pipe "/Game/Static/Meshes/Tuberia_Rota.Tuberia_Rota")))
  (set `/Game/Dynamic/Blueprints/VR_Template/GrabComponent.GrabType` "NewEnumerator4" (`self.PipeGrabComponent`))
  (`PrimitiveComponent.SetSimulatePhysics` (`self.Pipe`) true))