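; Pipe puzzle nut that is fixed by turning it until a steam leak stops.
; StartFixing plays the FixingNut timeline, which spins the nut mesh through several full yaw turns, and StopFixing reverses it from its current point, so interrupted progress unwinds.
; Finishing in the forward direction deactivates the steam effect and calls FixPipePuzzleActor.
; Both events do nothing once IsFixed is set.
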(event `self.ReceiveBeginPlay`
  (`parent.ReceiveBeginPlay`))

(event `StartFixing`
  (if (not (`self.isFixed`))
    (`|ExecutionSequence`
      (:`then_0`
        (bind (_direction _newtrack_0) (`Timeline|FixingNut` :!via `Stop` :!label _label)
          (:`Update`
            (`SceneComponent.K2_SetRelativeRotation` (`self.PipeNut`) (`KismetMathLibrary.MakeRotator` 0.0 0.0 (* _newtrack_0 (* 3.0 360.0))) false false))
          (:`Finished`
            (switch `ETimelineDirection` _direction
              (:`Forward`
                (`ActorComponent.Deactivate` (`self.NS_Steam`))
                (`self.FixPipePuzzleActor`))))))
      (:`then_1`
        (goto _label)))))

(event `StopFixing`
  (if (not (`self.isFixed`))
    (`|ExecutionSequence`
      (:`then_0`
        (goto _label :!via `Stop`))
      (:`then_1`
        (goto _label :!via `Reverse`)))))

(fn `UserConstructionScript`
  (`parent.UserConstructionScript`))