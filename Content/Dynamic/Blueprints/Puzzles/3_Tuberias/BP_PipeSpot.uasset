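; A pipe socket for a VR pipe puzzle, holding either a fixed pipe or a broken one to be replaced.
; The construction script sets mesh, grabbability and capsule visibility from the pipe type.
; Grabbing the broken pipe hands a spawned copy to the motion controller, while the original returns hidden as a straight pipe.
; When a straight BP_Pipe overlaps the free spot, it is destroyed, the hidden pipe reappears and the puzzle piece is fixed.
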(event `self.ReceiveBeginPlay`
  (bind _pipe (`self.Pipe`))
  ;[1 1 1] Begin Play
  (`parent.ReceiveBeginPlay`)
  (if (`self.isFixed`)
    (`self.CloseBeginOverlap`)
    (`self.CloseEndOverlap`)
    (else
      (`self.OpenBeginOverlap`)
      (`self.OpenEndOverlap`)
      (set `self.InitialPipeWorldTransform` (`SceneComponent.K2_GetComponentToWorld` _pipe))))
  (`PrimitiveComponent.SetSimulatePhysics` _pipe false)
  (`PrimitiveComponent.SetEnableGravity` _pipe true))

(event `self.CapsuleCollision.OnComponentBeginOverlap`
  (params (OverlappedComponent :type "PrimitiveComponent Object Reference") (OtherActor :type "Actor Object Reference") (OtherComp :type "PrimitiveComponent Object Reference") (OtherBodyIndex :type Integer) (bFromSweep :type Boolean) (SweepResult :type "HitResult Structure (by ref)"))
  ;[1 1 1] Has colocado una tubería arreglada nueva?
  (`/Engine/EditorBlueprintResources/StandardMacros.Gate` true :!label _label
    (:`Exit`
      (bind _asbp_pipe (cast `/Game/Dynamic/Blueprints/Puzzles/3_Tuberias/BP_Pipe` OtherActor))
      (if (and (== (`StaticMeshComponent.StaticMesh` (`/Game/Dynamic/Blueprints/Puzzles/3_Tuberias/BP_Pipe.Pipe` _asbp_pipe)) "/Game/Static/Meshes/Tuberia_Recta.Tuberia_Recta") (`self.isFree`))
        (set `self.isFree` false)
        (`self.K2_DestroyActor` _asbp_pipe)
        (`self.FixPipePuzzleActor`)
        (set `self.PipeType` "NewEnumerator0")
        (`SceneComponent.SetHiddenInGame` (`self.Pipe`) false false)))))

(event `OpenBeginOverlap`
  ;[1 1 1] Has colocado una tubería arreglada nueva?
  (goto _label :!via `Open`))

(event `CloseBeginOverlap`
  ;[1 1 1] Has colocado una tubería arreglada nueva?
  (goto _label :!via `Close`))

(event `self.CapsuleCollision.OnComponentEndOverlap`
  (params (OverlappedComponent :type "PrimitiveComponent Object Reference") (OtherActor :type "Actor Object Reference") (OtherComp :type "PrimitiveComponent Object Reference") (OtherBodyIndex :type Integer))
  ;[1 1 1] Al sacar la tubería rota
  (`/Engine/EditorBlueprintResources/StandardMacros.Gate` true :!label _label_2
    (:`Exit`
      (cast `/Game/Dynamic/Blueprints/Puzzles/3_Tuberias/BP_PipeSpot` (`ActorComponent.GetOwner` OtherComp))
      (set `self.isFree` true))))

(event `OpenEndOverlap`
  ;[1 1 1] Al sacar la tubería rota
  (goto _label_2 :!via `Open`))

(event `CloseEndOverlap`
  ;[1 1 1] Al sacar la tubería rota
  (goto _label_2 :!via `Close`))

(event `self.PipeGrabComponent.OnGrabbed`
  (bind _pipe (`self.Pipe`))
  (bind _pipegrabcomponent (`self.PipeGrabComponent`))
  (bind _motion_controller_ref (`self.Motion Controller Ref`))
  (bind (_initialpipeworldtransform_location _initialpipeworldtransform_rotation) (`KismetMathLibrary.BreakTransform` (`self.InitialPipeWorldTransform`)))
  (bind _as_vrpawn (`self.As VRPawn`))
  ;[1 1 1] Al soltar agarrar tubería...
  ;;[1 1 1] Al soltar la tubería, genera una de tipo Pipe que esté rota. Este componente de tubería se oculatará y se moverá al lugar inicial y se usará como tubería final al llevar una tubería arreglada. La generada se utilizará como un objeto mas del entorno
  ;;;[1 1 1] Delay minimo para evitar que el IA_Grab_Right del VRPawn, sobreescriba los nuevos valores
  (`KismetSystemLibrary.Delay` 0.01)
  (set `self.Motion Controller Ref` (`/Game/Dynamic/Blueprints/VR_Template/GrabComponent.MotionControllerRef` _pipegrabcomponent))
  (bind _asvrpawn (cast `/Game/Dynamic/Blueprints/VR_Template/VRPawn` (`GameplayStatics.GetPlayerPawn` 0)))
  (set `self.As VRPawn` _asvrpawn)
  (bind _breleased (`/Game/Dynamic/Blueprints/VR_Template/GrabComponent.TryRelease` _pipegrabcomponent))
  (if _breleased
    (set `/Game/Dynamic/Blueprints/VR_Template/GrabComponent.GrabType` "NewEnumerator0" (`self.PipeGrabComponent`))
    (`SceneComponent.SetHiddenInGame` _pipe true false)
    (`StaticMeshComponent.SetStaticMesh` _pipe "/Game/Static/Meshes/Tuberia_Recta.Tuberia_Recta")
    ;;;[1 1 1] Spawn new pipe on grabed actor transform
    (bind _returnvalue (`|SpawnActorFromClass` "/Game/Dynamic/Blueprints/Puzzles/3_Tuberias/BP_Pipe.BP_Pipe_C" (`SceneComponent.K2_GetComponentToWorld` _pipe) "Undefined" "MultiplyWithRoot" null null))
    (`SceneComponent.K2_SetWorldLocationAndRotation` _pipe _initialpipeworldtransform_location _initialpipeworldtransform_rotation false false)
    (`SceneComponent.SetMobility` _pipe "Static")
    (bind _pipegrabcomponent_2 (`/Game/Dynamic/Blueprints/Puzzles/3_Tuberias/BP_Pipe.PipeGrabComponent` _returnvalue))
    (bind _isheld (`/Game/Dynamic/Blueprints/VR_Template/GrabComponent.TryGrab` _pipegrabcomponent_2 _motion_controller_ref))
    (if _isheld
      (`StaticMeshComponent.SetStaticMesh` (`/Game/Dynamic/Blueprints/Puzzles/3_Tuberias/BP_Pipe.Pipe` _returnvalue) "/Game/Static/Meshes/Tuberia_Rota.Tuberia_Rota")
      (if (== _motion_controller_ref (`/Game/Dynamic/Blueprints/VR_Template/VRPawn.MotionControllerRightGrip` _as_vrpawn))
        (set `/Game/Dynamic/Blueprints/VR_Template/VRPawn.HeldComponentRight` _pipegrabcomponent_2 _as_vrpawn)
        (else
          (set `/Game/Dynamic/Blueprints/VR_Template/VRPawn.HeldComponentLeft` _pipegrabcomponent_2 _as_vrpawn)))
      (set `self.isFree` true))))

(fn `UserConstructionScript`
  (bind _pipe (`self.Pipe`))
  (switch `/Game/Dynamic/Blueprints/Puzzles/3_Tuberias/E_PipeTypes` (`self.PipeType`)
    (:`NewEnumerator0`
      (`StaticMeshComponent.SetStaticMesh` _pipe "/Game/Static/Meshes/Tuberia_Recta.Tuberia_Recta")
      (set `self.isFixed` true :!label _label)
      (set `/Game/Dynamic/Blueprints/VR_Template/GrabComponent.GrabType` "NewEnumerator0" (`self.PipeGrabComponent`))
      (`SceneComponent.SetVisibility` (`self.CapsuleCollision`) false false))
    (:`NewEnumerator1`
      (`StaticMeshComponent.SetStaticMesh` _pipe "/Game/Static/Meshes/Tuberia_Curva.Tuberia_Curva")
      (goto _label))
    (:`NewEnumerator2`
      (`StaticMeshComponent.SetStaticMesh` _pipe "/Game/Static/Meshes/Tuberia_Intersec.Tuberia_Intersec")
      (goto _label))
    (:`NewEnumerator3`
      (`StaticMeshComponent.SetStaticMesh` _pipe "/Game/Static/Meshes/Tuberia_Rota.Tuberia_Rota")
      (set `self.isFixed` false)
      (set `/Game/Dynamic/Blueprints/VR_Template/GrabComponent.GrabType` "NewEnumerator4" (`self.PipeGrabComponent`))
      (`SceneComponent.SetVisibility` (`self.CapsuleCollision`) true false))))