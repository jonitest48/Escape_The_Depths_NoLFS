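; BP_PipePuzzleActor is one piece of a pipe puzzle that tracks whether it has been fixed.
; On BeginPlay, an unfixed piece finds the BP_PipePuzzleManager in the level and adds itself to that manager's actor array.
; FixPipePuzzleActor sets IsFixed, writes the piece back into its array slot and has the manager check whether all pieces are fixed.
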(event `self.ReceiveBeginPlay`
  (if (not (`self.isFixed`))
    (bind _returnvalue (`GameplayStatics.GetActorOfClass` "/Game/Dynamic/Blueprints/Puzzles/3_Tuberias/BP_PipePuzzleManager.BP_PipePuzzleManager_C"))
    (bind _output_get (set `self.PipePuzzleManager` _returnvalue))
    (`KismetArrayLibrary.Array_Add` (`/Game/Dynamic/Blueprints/Puzzles/3_Tuberias/BP_PipePuzzleManager.PipePuzzleActors` _output_get) self)))

(event `FixPipePuzzleActor`
  (bind _pipepuzzleactors (`/Game/Dynamic/Blueprints/Puzzles/3_Tuberias/BP_PipePuzzleManager.PipePuzzleActors` (`self.PipePuzzleManager`)))
  (set `self.isFixed` true)
  (`KismetArrayLibrary.Array_Set` _pipepuzzleactors (`KismetArrayLibrary.Array_Find` _pipepuzzleactors self) self)
  (`/Game/Dynamic/Blueprints/Puzzles/3_Tuberias/BP_PipePuzzleManager.CheckAllFixed` (`self.PipePuzzleManager`)))

(fn `UserConstructionScript`)