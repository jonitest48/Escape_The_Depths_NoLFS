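; Keypad color-sequence puzzle actor that randomly generates a color and number clue for each tagged hint mesh.
; On BeginPlay it builds the sequence, using a random non-looping MultiGate for non-repeating colors.
; It spawns a matching BP_PuzzleFigure per entry at an unused random BP_FigureSpawnLocation, re-rolling on collisions.
; When BP_EventManager signals power on, the hint screens switch to their sequence colors.
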(event `Bind_TurnPowerOn`
  ;[1 1 1] EventManager
  (`self.TurnPowerOn`))

(event `/Game/Dynamic/Blueprints/Interfaces/BPI_LightPowered.TurnPowerOn`
  ;[1 1 1] On Turn Power On
  (for (_array_element _array_index) (`self.colorHints`)
    (bind _asstatic_mesh_component (cast `StaticMeshComponent` _array_element))
    (switch `/Game/Dynamic/Blueprints/Puzzles/4_FigurasGeometricas/E_FigureSeqColors` (`|GetArrayItem` (`self.sequenceColors`) _array_index)
      (:`NewEnumerator0`
        (`PrimitiveComponent.SetMaterial` _asstatic_mesh_component 0 "/Game/Dynamic/Materials/MI/MI_ScreenPink.MI_ScreenPink"))
      (:`NewEnumerator1`
        (`PrimitiveComponent.SetMaterial` _asstatic_mesh_component 0 "/Game/Dynamic/Materials/MI/MI_ScreenSkyBlue.MI_ScreenSkyBlue"))
      (:`NewEnumerator2`
        (`PrimitiveComponent.SetMaterial` _asstatic_mesh_component 0 "/Game/Dynamic/Materials/MI/MI_ScreenLime.MI_ScreenLime"))
      (:`NewEnumerator3`
        (`PrimitiveComponent.SetMaterial` _asstatic_mesh_component 0 "/Game/Dynamic/Materials/MI/MI_ScreenPurple.MI_ScreenPurple"))
      (:`NewEnumerator4`
        (`PrimitiveComponent.SetMaterial` _asstatic_mesh_component 0 "/Engine/TemplateResources/MI_Template_BaseOrange_Metal.MI_Template_BaseOrange_Metal")))))

(event `self.ReceiveBeginPlay`
  (bind _sequencecolors (`self.sequenceColors`))
  ;[1 1 1] Get FigureSpawnLocations
  (bind _outactors (`GameplayStatics.GetAllActorsOfClass` "/Game/Dynamic/Blueprints/Puzzles/4_FigurasGeometricas/Figures/BP_FigureSpawnLocation.BP_FigureSpawnLocation_C"))
  (set `self.FigureSpawnLocations` _outactors)
  ;[1 1 1] Get TextHints
  (set `self.textHints` (`self.K2_GetComponentsByClass` self "/Script/Engine.TextRenderComponent"))
  (`|ExecutionSequence`
    (:`then_0`
      ;[1 1 1] EventManager
      (bind _returnvalue (`GameplayStatics.GetActorOfClass` "/Game/Dynamic/Blueprints/BP_EventManager.BP_EventManager_C"))
      (bind _output_get (set `self.EventManager` _returnvalue))
      (add `/Game/Dynamic/Blueprints/BP_EventManager.ED_TurnPowerOn` _output_get (delegate `Bind_TurnPowerOn`)))
    (:`then_1`
      ;[1 1 1] Generacion de sequencia de colores y numeros
      (bind _output_get_2 (set `self.colorHints` (`self.GetComponentsByTag` self "/Script/Engine.StaticMeshComponent" "colorHint")))
      (for _ _output_get_2
        (`KismetArrayLibrary.Array_Add` (`self.sequenceValue`) (`KismetMathLibrary.RandomIntegerInRange` 3 8))
        (`|MultiGate` true
          (:`Out 0`
            (`KismetArrayLibrary.Array_Add` _sequencecolors "NewEnumerator0"))
          (:`Out 1`
            (`KismetArrayLibrary.Array_Add` _sequencecolors "NewEnumerator1"))
          (:`Out 2`
            (`KismetArrayLibrary.Array_Add` _sequencecolors "NewEnumerator2"))
          (:`Out 3`
            (`KismetArrayLibrary.Array_Add` _sequencecolors "NewEnumerator3"))
          (:`Out 4`
            (`KismetArrayLibrary.Array_Add` _sequencecolors "NewEnumerator4"))))
      (for (_ _array_index) _output_get_2
        (`self.SpawnFigure` (`|GetArrayItem` (`self.sequenceColors`) _array_index) (`|GetArrayItem` (`self.sequenceValue`) _array_index))))))

(fn `getIsPowered`
  (returns (isPowered :type Boolean))
  (return false))

(fn `SetFigureProperties`
  (params (Target :type "/Game/Dynamic/Blueprints/Puzzles/4_FigurasGeometricas/Figures/BP_PuzzleFigure Object Reference") (FigureType :type "/Game/Dynamic/Blueprints/Puzzles/4_FigurasGeometricas/Figures/E_FigureType_ColorKeypad Enum" :default "NewEnumerator0") (ScaleMultiplier :type "Float (double-precision)") (Color :type "/Game/Dynamic/Blueprints/Puzzles/4_FigurasGeometricas/E_FigureSeqColors Enum" :default "NewEnumerator0") (Valor :type Integer) (RandomSpawnerNumber :type "Integer (by ref)"))
  (`/Game/Dynamic/Blueprints/Puzzles/4_FigurasGeometricas/Figures/BP_PuzzleFigure.UpdateFigurePuzzleValues` Target FigureType ScaleMultiplier Color Valor)
  (`KismetArrayLibrary.Array_Add` (`self.AlreadySpawnedIn`) RandomSpawnerNumber))

(fn `SpawnFigure`
  (params (Color :type "/Game/Dynamic/Blueprints/Puzzles/4_FigurasGeometricas/E_FigureSeqColors Enum" :default "NewEnumerator0") (Valor :type Integer))
  (locals (randomSpawnerNumber :type Integer))
  (bind _randomspawnernumber (`local.randomSpawnerNumber`))
  (bind _figurespawnlocations (`self.FigureSpawnLocations`))
  (bind _output (`|GetArrayItem` _figurespawnlocations (`local.randomSpawnerNumber`)))
  (bind _returnvalue (`KismetMathLibrary.RandomIntegerInRange` 0 (`KismetArrayLibrary.Array_LastIndex` _figurespawnlocations)))
  (bind _rootcomponent (`Actor.RootComponent` _output))
  ;[1 1 1] Comprueba que existen localizaciones de spawn en el nivel y elegirá un punto aleatorio por cada número de la secuencia generado para spawnear una figura en esa localizacion. Mientras que el numero aleatorio generado ya haya sido utilizado, generará indefinidamente otro número hasta que no hayan coincidencias
  (if (>= (`KismetArrayLibrary.Array_Length` _figurespawnlocations) 4)
    (set `local.randomSpawnerNumber` _returnvalue)
    (while (!= (`KismetArrayLibrary.Array_Find` (`self.AlreadySpawnedIn`) _randomspawnernumber) -1)
      (set `local.randomSpawnerNumber` _returnvalue))
    (bind _returnvalue_2 (`|SpawnActorFromClass` "/Game/Dynamic/Blueprints/Puzzles/4_FigurasGeometricas/Figures/BP_PuzzleFigure.BP_PuzzleFigure_C" (`KismetMathLibrary.MakeTransform` (`SceneComponent.K2_GetComponentLocation` _rootcomponent) (`SceneComponent.K2_GetComponentRotation` _rootcomponent)) "Undefined" "MultiplyWithRoot" null null))
    (`self.SetFigureProperties` _returnvalue_2 (`/Game/Dynamic/Blueprints/Puzzles/4_FigurasGeometricas/Figures/BP_FigureSpawnLocation.FigureType` _output) (`/Game/Dynamic/Blueprints/Puzzles/4_FigurasGeometricas/Figures/BP_FigureSpawnLocation.ScaleMultiplier` _output) Color Valor _randomspawnernumber)))

(fn `UserConstructionScript`)