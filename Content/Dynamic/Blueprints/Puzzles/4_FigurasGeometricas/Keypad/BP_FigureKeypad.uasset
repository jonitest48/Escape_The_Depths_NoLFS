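; Keypad for a geometric-figures puzzle, where the player enters a code that must match the generated sequence.
; On BeginPlay it registers itself with child buttons and binds to the color-sequence actor's EventManager to set its powered flag.
; Each press fills the matching text hint; at full length the code is checked.
; A match turns buttons green, deactivates them and notifies BP_EndGamePad; a mismatch plays a sound and resets input.
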(event `self.ReceiveBeginPlay`
  ;[1 1 1] Recoge todos los actores hijos y, solo los botones, los añade a un array y les asigna a la variable Father Figure Key Pad este blueprint (self)
  (for _array_element (`self.K2_GetComponentsByClass` self "/Script/Engine.ChildActorComponent")
    (bind _childactor (`ChildActorComponent.ChildActor` _array_element))
    (bind _asbp_key_pad_button (cast `/Game/Dynamic/Blueprints/Puzzles/4_FigurasGeometricas/Keypad/BP_KeyPadButton` _childactor)
      (:`then`
        (`KismetArrayLibrary.Array_Add` (`self.AllButtons`) _asbp_key_pad_button)
        (set `/Game/Dynamic/Blueprints/Puzzles/4_FigurasGeometricas/Keypad/BP_KeyPadButton.Father_FigureKeyPad` self _asbp_key_pad_button))
      (:`CastFailed`
        (bind _asbp_key_pad_color_seq (cast `/Game/Dynamic/Blueprints/Puzzles/4_FigurasGeometricas/Keypad/BP_KeyPadColorSeq` _childactor))
        (bind _output_get (set `self.As BP Key Pad Color Seq` _asbp_key_pad_color_seq))
        (bind _eventmanager (`/Game/Dynamic/Blueprints/Puzzles/4_FigurasGeometricas/Keypad/BP_KeyPadColorSeq.EventManager` _output_get))
        (`/Engine/EditorBlueprintResources/StandardMacros.IsValid` _eventmanager :!label _label
          (:`Is Valid`
            (bind _output_get_2 (set `self.Event Manager` _eventmanager))
            (add `/Game/Dynamic/Blueprints/BP_EventManager.ED_TurnPowerOn` _output_get_2 (delegate `Turn Power On`)))
          (:`Is Not Valid`
            (goto _label)))))))

(event `Turn Power On`
  ;[1 1 1] Recoge todos los actores hijos y, solo los botones, los añade a un array y les asigna a la variable Father Figure Key Pad este blueprint (self)
  (set `self.IsPowered` true))

(fn `ButtonPressed`
  (params (PressedButonValue :type Integer))
  (locals (AuxTextRender :type "TextRenderComponent Object Reference"))
  (bind _usersequence (`self.UserSequence`))
  (bind _returnvalue (`KismetArrayLibrary.Array_LastIndex` _usersequence))
  ;[1 1 1] Cambiar número en orden de secuencia
  (`KismetArrayLibrary.Array_Add` _usersequence PressedButonValue)
  (bind _asbp_key_pad_color_seq (cast `/Game/Dynamic/Blueprints/Puzzles/4_FigurasGeometricas/Keypad/BP_KeyPadColorSeq` (`ChildActorComponent.ChildActor` (`self.ColorHintLights`))))
  (for _array_element (`/Game/Dynamic/Blueprints/Puzzles/4_FigurasGeometricas/Keypad/BP_KeyPadColorSeq.textHints` _asbp_key_pad_color_seq)
    (if (`KismetStringLibrary.EqualEqual_StrStr` (`KismetSystemLibrary.GetObjectName` _array_element) (`KismetStringLibrary.Concat_StrStr` "Text" (`KismetStringLibrary.Conv_IntToString` (+ _returnvalue 1))))
      (`TextRenderComponent.K2_SetText` _array_element (`KismetTextLibrary.Conv_IntToText` (`local.PressedButonValue`)))
      (break)))
  ;[1 1 1] Si es el último boton pulsado de la secuencia ...
  (if (== (`KismetArrayLibrary.Array_LastIndex` (`/Game/Dynamic/Blueprints/Puzzles/4_FigurasGeometricas/Keypad/BP_KeyPadColorSeq.sequenceValue` _asbp_key_pad_color_seq)) _returnvalue)
    (bind _iscorrect (`self.CheckSequence`))
    (if _iscorrect
      (for _array_element_2 (`self.AllButtons`)
        (`PrimitiveComponent.SetMaterial` (`/Game/Dynamic/Blueprints/Puzzles/4_FigurasGeometricas/Keypad/BP_KeyPadButton.Button` _array_element_2) 0 "/Engine/EngineDebugMaterials/VertexColorViewMode_GreenOnly.VertexColorViewMode_GreenOnly")
        (`/Game/Dynamic/Blueprints/Puzzles/4_FigurasGeometricas/Keypad/BP_KeyPadButton.DeactivateButton` _array_element_2))
      (bind _returnvalue_2 (`GameplayStatics.GetActorOfClass` "/Game/Dynamic/Blueprints/Puzzles/5_EndGame/BP_EndGamePad.BP_EndGamePad_C"))
      (`/Game/Dynamic/Blueprints/Puzzles/5_EndGame/BP_EndGamePad.CompletePuzzle` _returnvalue_2 (`self.PuzzleNumber`))
      (else
        (`self.ResetUserSequence`)))))

(fn `CheckSequence`
  (returns (isCorrect :type Boolean))
  (locals (NewLocalVar :type Boolean :default true))
  (bind _sequencevalue (`/Game/Dynamic/Blueprints/Puzzles/4_FigurasGeometricas/Keypad/BP_KeyPadColorSeq.sequenceValue` (`self.As BP Key Pad Color Seq`)))
  ;[1 1 1] Compureba que lo generado por la maquina y lo introducido por el usuario es el mismo codigo y devuelve el boolean correspondiente
  (`KismetSystemLibrary.PrintString` "Secuencia Generada" true true (struct :`R` 1.0 :`B` 0.050593 :`A` 1.0) 20.0)
  (for (_array_element _array_index) _sequencevalue
    (`KismetSystemLibrary.PrintString` (`KismetStringLibrary.Concat_StrStr` (`KismetStringLibrary.Conv_IntToString` _array_index) "-" (`KismetStringLibrary.Conv_IntToString` _array_element)) true true (struct :`R` 1.0 :`B` 0.050593 :`A` 1.0) 20.0))
  (`KismetSystemLibrary.PrintString` "Secuencia Introducida" true true (struct :`R` 0.506762 :`G` 0.113053 :`B` 1.0 :`A` 1.0) 20.0)
  (for (_array_element_2 _array_index_2) _
    (`KismetSystemLibrary.PrintString` (`KismetStringLibrary.Concat_StrStr` (`KismetStringLibrary.Conv_IntToString` _array_index_2) "-" (`KismetStringLibrary.Conv_IntToString` _array_element_2)) true true (struct :`R` 0.861232 :`G` 0.133161 :`B` 1.0 :`A` 1.0) 20.0))
  (for (_array_element_3 _array_index_3) _sequencevalue
    (if (not (== _array_element_3 (`|GetArrayItem` (`self.UserSequence`) _array_index_3)))
      (set `local.NewLocalVar` false)
      (break)))
  (return (`local.NewLocalVar`)))

(fn `ResetUserSequence`
  (`GameplayStatics.PlaySoundAtLocation` "/Engine/EditorSounds/Notifications/CompileFailed_Cue.CompileFailed_Cue" (`SceneComponent.K2_GetComponentLocation` (`self.DefaultSceneRoot`)) (struct) 1.0 1.0 0.0 null null null null)
  (`KismetArrayLibrary.Array_Clear` (`self.UserSequence`))
  (for _array_element (`/Game/Dynamic/Blueprints/Puzzles/4_FigurasGeometricas/Keypad/BP_KeyPadColorSeq.textHints` (`self.As BP Key Pad Color Seq`))
    (`TextRenderComponent.K2_SetText` _array_element "0")))

(fn `UserConstructionScript`)