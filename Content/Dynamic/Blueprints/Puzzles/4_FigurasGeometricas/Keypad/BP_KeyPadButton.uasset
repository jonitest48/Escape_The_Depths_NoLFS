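; BP_KeyPadButton is a VR keypad button for a geometric figures puzzle, displaying its numeric Value as text.
; A VRPawn overlap sinks the button, swaps its material and reports Value to FatherFigureKeyPad.
; With a valid keypad, it springs back after a half-second delay.
; DeactivateButton closes the gate on pressing and, after a short delay, the gate on unpressing.
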(event `/Game/Dynamic/Blueprints/Interfaces/BPI_Button.Unpress`
  (`/Engine/EditorBlueprintResources/StandardMacros.Gate` false :!label _label
    (:`Exit`
      (if (`self.isButtonPressed`)
        (`self.AnimacionBoton`
          (:`Completed`
            (`PrimitiveComponent.SetMaterial` (`self.Button`) 0 "/Engine/MapTemplates/Materials/BasicAsset02.BasicAsset02")
            (set `self.isButtonPressed` false)))))))

(event `DeactivateButton`
  (`|ExecutionSequence`
    (:`then_0`
      (`KismetSystemLibrary.Delay` 0.6)
      (goto _label :!via `Close`))
    (:`then_1`
      (goto _label_2 :!via `Close`))))

(event `/Game/Dynamic/Blueprints/Interfaces/BPI_Button.Press`
  (`/Engine/EditorBlueprintResources/StandardMacros.Gate` false :!label _label_2
    (:`Exit`
      (if (not (`self.isButtonPressed`))
        (`self.AnimacionBoton`
          (:`Completed`
            (`PrimitiveComponent.SetMaterial` (`self.Button`) 0 "/Engine/BasicShapes/BasicShapeMaterial.BasicShapeMaterial")
            (set `self.isButtonPressed` true)
            (`/Engine/EditorBlueprintResources/StandardMacros.IsValid` (`self.Father_FigureKeyPad`)
              (:`Is Valid`
                (`/Game/Dynamic/Blueprints/Puzzles/4_FigurasGeometricas/Keypad/BP_FigureKeypad.ButtonPressed` (`self.Father_FigureKeyPad`) (`self.Value`))
                (`KismetSystemLibrary.Delay` 0.5)
                (`self.Unpress`)))))))))

(event `self.ButtonCollision.OnComponentBeginOverlap`
  (params (OverlappedComponent :type "PrimitiveComponent Object Reference") (OtherActor :type "Actor Object Reference") (OtherComp :type "PrimitiveComponent Object Reference") (OtherBodyIndex :type Integer) (bFromSweep :type Boolean) (SweepResult :type "HitResult Structure (by ref)"))
  (cast `/Game/Dynamic/Blueprints/VR_Template/VRPawn` OtherActor)
  (if (not (`self.isButtonPressed`))
    (`self.Press`)))

(fn `isPressed`
  (returns (isPressed :type Boolean))
  (return (`self.isButtonPressed`)))

(fn `SetValueText`
  (`TextRenderComponent.K2_SetText` (`self.ValueText`) (`KismetTextLibrary.Conv_IntToText` (`self.Value`))))

(fn `UserConstructionScript`
  (`self.SetValueText`))