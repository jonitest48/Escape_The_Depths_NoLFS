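; BP_FigureSpawnLocation is an actor in the geometric figures puzzle that, judging by its name, marks where a figure spawns.
; Its construction script picks the static mesh from FigureType, covering photo, book, cup and drill props.
; It then multiplies the mesh component's relative scale by ScaleMultiplier, and holds no other graph logic.
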(fn `UserConstructionScript`
  (bind _staticmesh (`self.StaticMesh`))
  (bind _staticmesh_2 (`self.StaticMesh`))
  (switch `/Game/Dynamic/Blueprints/Puzzles/4_FigurasGeometricas/Figures/E_FigureType_ColorKeypad` (`self.FigureType`)
    (:`NewEnumerator0`
      (`StaticMeshComponent.SetStaticMesh` _staticmesh "/Game/Static/Meshes/SM_Foto.SM_Foto"))
    (:`NewEnumerator1`
      (`StaticMeshComponent.SetStaticMesh` _staticmesh "/Game/Static/Meshes/SM_Libro.SM_Libro"))
    (:`NewEnumerator2`
      (`StaticMeshComponent.SetStaticMesh` _staticmesh "/Game/Static/Meshes/SM_Taza.SM_Taza"))
    (:`NewEnumerator3`
      (`StaticMeshComponent.SetStaticMesh` _staticmesh "/Game/Static/Meshes/Taladro/SM_TaladroV2.SM_TaladroV2")))
  (`SceneComponent.SetRelativeScale3D` _staticmesh_2 (* (`SceneComponent.RelativeScale3D` _staticmesh_2) (`self.ScaleMultiplier`))))