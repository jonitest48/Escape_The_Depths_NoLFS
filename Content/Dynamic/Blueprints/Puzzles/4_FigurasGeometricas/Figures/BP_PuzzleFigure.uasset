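; Puzzle figure actor for the geometric figures puzzle, shown as a photo, book, mug or drill according to FigureType.
; The construction script picks the mesh and applies a scale multiplier to all but the drill.
; SetColorAndValue only stores color and value, as its text and screen-material updates are disconnected.
; On BeginPlay the drill only prints a debug message; spawning the functional BP_PipeFixer tool is not wired up.
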(event `self.ReceiveBeginPlay`
  (switch `/Game/Dynamic/Blueprints/Puzzles/4_FigurasGeometricas/Figures/E_FigureType_ColorKeypad` (`self.FigureType`)
    (:`NewEnumerator3`
      (`KismetSystemLibrary.PrintString` "SPAWN TALADRO"))))

(fn `SetColorAndValue`
  (params (Color :type "/Game/Dynamic/Blueprints/Puzzles/4_FigurasGeometricas/E_FigureSeqColors Enum" :default "NewEnumerator0") (Valor :type Integer))
  (set `self.Color` Color)
  (set `self.Valor` Valor))

(fn `UserConstructionScript`
  (bind _figure (`self.Figure`))
  (bind _figure_2 (`self.Figure`))
  (switch `/Game/Dynamic/Blueprints/Puzzles/4_FigurasGeometricas/Figures/E_FigureType_ColorKeypad` (`self.FigureType`)
    (:`NewEnumerator0`
      (`StaticMeshComponent.SetStaticMesh` _figure "/Game/Static/Meshes/SM_Foto.SM_Foto")
      (`SceneComponent.SetRelativeScale3D` _figure_2 (* (`SceneComponent.RelativeScale3D` _figure_2) (`self.ScaleMultiplier`)) :!label _label))
    (:`NewEnumerator1`
      (`StaticMeshComponent.SetStaticMesh` _figure "/Game/Static/Meshes/SM_Libro.SM_Libro")
      (goto _label))
    (:`NewEnumerator2`
      (`StaticMeshComponent.SetStaticMesh` _figure "/Game/Static/Meshes/SM_Taza.SM_Taza")
      (goto _label))
    (:`NewEnumerator3`
      ;[1 1 1] En el Begin Play, en caso de ser taladro, se autodestruirá y generará la BP de la herramienta funcional
      (`StaticMeshComponent.SetStaticMesh` _figure "/Game/Static/Meshes/SM_Taladro.SM_Taladro"))))