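; BP_PuzzleFigure is a figure piece for a geometric-figures puzzle, carrying a color and a numeric value.
; SetColorAndValue stores both, shows the value on its TextRender and switches on the color enum to set the Plane's material.
; Pink, sky blue, lime and purple use screen materials, while orange uses a template metal material.
; The construction script is empty, so the look is applied only when that function is called.
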(fn `SetColorAndValue`
  (params (Color :type "/Game/Dynamic/Blueprints/Puzzles/FigurasGeometricas/E_FigureSeqColors Enum" :default "NewEnumerator0") (Valor :type Integer))
  (bind _plane (`self.Plane`))
  (set `self.Color` Color)
  (set `self.Valor` Valor)
  (`TextRenderComponent.K2_SetText` (`self.TextRender`) (`KismetTextLibrary.Conv_IntToText` (`self.Valor`)))
  (switch `/Game/Dynamic/Blueprints/Puzzles/FigurasGeometricas/E_FigureSeqColors` (`self.Color`)
    (:`NewEnumerator0`
      (`PrimitiveComponent.SetMaterial` _plane 0 "/Game/Static/Materials/MI/MI_ScreenPink.MI_ScreenPink"))
    (:`NewEnumerator1`
      (`PrimitiveComponent.SetMaterial` _plane 0 "/Game/Static/Materials/MI/MI_ScreenSkyBlue.MI_ScreenSkyBlue"))
    (:`NewEnumerator2`
      (`PrimitiveComponent.SetMaterial` _plane 0 "/Game/Static/Materials/MI/MI_ScreenLime.MI_ScreenLime"))
    (:`NewEnumerator3`
      (`PrimitiveComponent.SetMaterial` _plane 0 "/Game/Static/Materials/MI/MI_ScreenPurple.MI_ScreenPurple"))
    (:`NewEnumerator4`
      (`PrimitiveComponent.SetMaterial` _plane 0 "/Engine/TemplateResources/MI_Template_BaseOrange_Metal.MI_Template_BaseOrange_Metal"))))

(fn `UserConstructionScript`)