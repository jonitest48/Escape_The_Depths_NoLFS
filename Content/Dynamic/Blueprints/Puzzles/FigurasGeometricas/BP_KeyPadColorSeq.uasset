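; Keypad puzzle Blueprint that generates a random color and number sequence on BeginPlay.
; For each mesh tagged "colorHint", it stores a random integer and draws one of five colors through a random, non-looping MultiGate, so colors never repeat.
; It then switches on each stored color to set that mesh's material.
; Text render components are cached as hints but never written, and no input checking is present.
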(event `self.ReceiveBeginPlay`
  (bind _sequencecolors (`self.sequenceColors`))
  ;[1 1 1] Get TextHints
  (set `self.textHints` (`self.K2_GetComponentsByClass` self "/Script/Engine.TextRenderComponent"))
  ;[1 1 1] Generacion de sequencia de colores y numeros
  (bind _output_get (set `self.colorHints` (`self.GetComponentsByTag` self "/Script/Engine.StaticMeshComponent" "colorHint")))
  (for _ _output_get
    (`KismetArrayLibrary.Array_Add` (`self.sequenceValue`) (`KismetMathLibrary.RandomIntegerInRange` 3 8))
    (`|MultiGate` true
      (:`Out 0`
        (`KismetArrayLibrary.Array_Add` _sequencecolors "NewEnumerator0"))
      (:`Out 1`
        (`KismetArrayLibrary.Array_Add` _sequencecolors "NewEnumerator1"))
      (:`Out 2`
        (`KismetArrayLibrary.Array_Add` _sequencecolors "NewEnumerator2"))
      (:`Out 3`
        (`KismetArrayLibrary.Array_Add` _sequencecolors "NewEnumerator3"))
      (:`Out 4`
        (`KismetArrayLibrary.Array_Add` _sequencecolors "NewEnumerator4"))))
  (for (_array_element _array_index) _output_get
    (bind _asstatic_mesh_component (cast `StaticMeshComponent` _array_element))
    (switch `/Game/Dynamic/Blueprints/Puzzles/FigurasGeometricas/E_FigureSeqColors` (`|GetArrayItem` (`self.sequenceColors`) _array_index)
      (:`NewEnumerator0`
        (`PrimitiveComponent.SetMaterial` _asstatic_mesh_component 0 null))
      (:`NewEnumerator1`
        (`PrimitiveComponent.SetMaterial` _asstatic_mesh_component 0 null))
      (:`NewEnumerator2`
        (`PrimitiveComponent.SetMaterial` _asstatic_mesh_component 0 null))
      (:`NewEnumerator3`
        (`PrimitiveComponent.SetMaterial` _asstatic_mesh_component 0 null))
      (:`NewEnumerator4`
        (`PrimitiveComponent.SetMaterial` _asstatic_mesh_component 0 null)))))

(fn `UserConstructionScript`)