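; BP_FigureKeypad is a keypad actor for the geometric figures puzzle, built from BP_KeyPadButton child actors.
; On BeginPlay it gathers each button from its child actor components into an array and sets itself as that button's parent keypad.
; ButtonPressed takes a value and only prints it with a debug message, with no puzzle logic yet.
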(event `self.ReceiveBeginPlay`
  (for _array_element (`self.K2_GetComponentsByClass` self "/Script/Engine.ChildActorComponent")
    (bind _asbp_key_pad_button (cast `/Game/Dynamic/Blueprints/Puzzles/FigurasGeometricas/BP_KeyPadButton` (`ChildActorComponent.ChildActor` _array_element)))
    (`KismetArrayLibrary.Array_Add` (`self.AllButtons`) _asbp_key_pad_button)
    (set `/Game/Dynamic/Blueprints/Puzzles/FigurasGeometricas/BP_KeyPadButton.Father_FigureKeyPad` self _asbp_key_pad_button)))

(fn `ButtonPressed`
  (params (NewParam :type Integer))
  (`KismetSystemLibrary.PrintString` (`KismetStringLibrary.Conv_IntToString` NewParam))
  (`KismetSystemLibrary.PrintString` "Tecla pulsada con valor"))

(fn `UserConstructionScript`)