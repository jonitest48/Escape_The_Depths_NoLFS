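; Geometric-figure keypad puzzle that checks the player's button sequence against a code held by a color-sequence display.
; On BeginPlay it gathers child-actor buttons, hands each a reference to itself, and caches the display.
; Each press appends a value and updates that position's hint text.
; A full-length match turns all buttons green and deactivates them; a mismatch plays an error sound and clears input and hints.
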(event `self.ReceiveBeginPlay`
  ;[1 1 1] Recoge todos los actores hijos y, solo los botones, los añade a un array y les asigna a la variable Father Figure Key Pad este blueprint (self)
  (for _array_element (`self.K2_GetComponentsByClass` self "/Script/Engine.ChildActorComponent")
    (bind _childactor (`ChildActorComponent.ChildActor` _array_element))
    (bind _asbp_key_pad_button (cast `/Game/Dynamic/Blueprints/Puzzles/FigurasGeometricas/Keypad/BP_KeyPadButton` _childactor)
      (:`then`
        (`KismetArrayLibrary.Array_Add` (`self.AllButtons`) _asbp_key_pad_button)
        (set `/Game/Dynamic/Blueprints/Puzzles/FigurasGeometricas/Keypad/BP_KeyPadButton.Father_FigureKeyPad` self _asbp_key_pad_button))
      (:`CastFailed`
        (bind _asbp_key_pad_color_seq (cast `/Game/Dynamic/Blueprints/Puzzles/FigurasGeometricas/Keypad/BP_KeyPadColorSeq` _childactor))
        (set `self.As BP Key Pad Color Seq` _asbp_key_pad_color_seq)))))

(fn `ButtonPressed`
  (params (PressedButonValue :type Integer))
  (bind _usersequence (`self.UserSequence`))
  (bind _returnvalue (`KismetArrayLibrary.Array_LastIndex` _usersequence))
  ;[1 1 1] Cambiar número en orden de secuencia
  (`KismetArrayLibrary.Array_Add` _usersequence PressedButonValue)
  (bind _asbp_key_pad_color_seq (cast `/Game/Dynamic/Blueprints/Puzzles/FigurasGeometricas/Keypad/BP_KeyPadColorSeq` (`ChildActorComponent.ChildActor` (`self.ColorHintLights`))))
  (`TextRenderComponent.K2_SetText` (`|GetArrayItem` (`/Game/Dynamic/Blueprints/Puzzles/FigurasGeometricas/Keypad/BP_KeyPadColorSeq.textHints` _asbp_key_pad_color_seq) _returnvalue) (`KismetTextLibrary.Conv_IntToText` (`local.PressedButonValue`)))
  (if (== (`KismetArrayLibrary.Array_LastIndex` (`/Game/Dynamic/Blueprints/Puzzles/FigurasGeometricas/Keypad/BP_KeyPadColorSeq.sequenceValue` _asbp_key_pad_color_seq)) _returnvalue)
    (bind _iscorrect (`self.CheckSequence`))
    (if _iscorrect
      (for _array_element (`self.AllButtons`)
        (`PrimitiveComponent.SetMaterial` (`/Game/Dynamic/Blueprints/Puzzles/FigurasGeometricas/Keypad/BP_KeyPadButton.Button` _array_element) 0 "/Engine/EngineDebugMaterials/VertexColorViewMode_GreenOnly.VertexColorViewMode_GreenOnly")
        (`/Game/Dynamic/Blueprints/Puzzles/FigurasGeometricas/Keypad/BP_KeyPadButton.DeactivateButton` _array_element))
      (else
        (`self.ResetUserSequence`)))))

(fn `CheckSequence`
  (returns (isCorrect :type Boolean))
  (locals (NewLocalVar :type Boolean :default true))
  ;[1 1 1] Compureba que lo generado por la maquina y lo introducido por el usuario es el mismo codigo y devuelve el boolean correspondiente
  (for (_array_element _array_index) (`/Game/Dynamic/Blueprints/Puzzles/FigurasGeometricas/Keypad/BP_KeyPadColorSeq.sequenceValue` (`self.As BP Key Pad Color Seq`))
    (if (not (== _array_element (`|GetArrayItem` (`self.UserSequence`) _array_index)))
      (set `local.NewLocalVar` false)
      (break)))
  (return (`local.NewLocalVar`)))

(fn `ResetUserSequence`
  (`GameplayStatics.PlaySoundAtLocation` "/Engine/EditorSounds/Notifications/CompileFailed_Cue.CompileFailed_Cue" (`SceneComponent.K2_GetComponentLocation` (`self.DefaultSceneRoot`)) (struct) 1.0 1.0 0.0 null null null null)
  (`KismetArrayLibrary.Array_Clear` (`self.UserSequence`))
  (for _array_element (`/Game/Dynamic/Blueprints/Puzzles/FigurasGeometricas/Keypad/BP_KeyPadColorSeq.textHints` (`self.As BP Key Pad Color Seq`))
    (`TextRenderComponent.K2_SetText` _array_element "0")))

(fn `UserConstructionScript`)