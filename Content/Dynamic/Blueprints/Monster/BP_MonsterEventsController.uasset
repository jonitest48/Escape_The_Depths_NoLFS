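; Monster events controller that periodically triggers a random Lights, Horn or Silence event, preceded by a sonar warning.
; Timelines scaled by play rate act as timers: the sonar starts a minute before each event and pings progressively faster.
; A random looping MultiGate picks the event, but only Lights calls BP_EventManager; Horn and Silence just print and count down.
; Countdown completion restarts the cycle, as do Stop events, whose EventManager bindings are never executed.
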(event `self.ReceiveBeginPlay`
  ;[1 1 1] On Begin | Enable Monster Event Timer
  (set `self.TimeBetweenEventInSeconds` (* 60.0 (`self.MonsterEventMinutes`)))
  (set `self.EventCountdownSeconds` (* 60.0 (`self.EventCountdownMinutes`)))
  (bind _returnvalue (`GameplayStatics.GetActorOfClass` "/Game/Dynamic/Blueprints/BP_EventManager.BP_EventManager_C"))
  (bind _output_get (set `self.EventManager` _returnvalue))
  (`self.StartMonsterEvents`))

(event `InitiateSonar`
  (bind _sonarsound (`self.SonarSound`))
  (bind _returnvalue (`TimelineComponent.GetPlayRate` _sonarsound))
  ;[1 1 1] SONAR
  (`TimelineComponent.SetPlayRate` (`self.SonarSound`) 1.0)
  (`Timeline|SonarSound` :!via `PlayFromStart`
    (:`SonarSoundTrack`
      (if (not (>= _returnvalue 4.0))
        (`TimelineComponent.SetPlayRate` _sonarsound (+ _returnvalue 0.08)))
      (`GameplayStatics.PlaySound2D` "/Game/Dynamic/Audio/submarine-sonar-38243_Edited.submarine-sonar-38243_Edited" 1.0 1.0 0.0 null null))))

(event `StartMonsterEvents`
  ;[1 1 1] START MONSTER EVENTS ON POWER ON
  (`|ExecutionSequence`
    (:`then_0`
      (`TimelineComponent.SetPlayRate` (`self.InitiateMonsterEventCountdown`) (/ 1.0 (`self.MonsterEventMinutes`)))
      (`Timeline|InitiateMonsterEventCountdown` :!via `PlayFromStart`
        (:`Finished`
          (`self.DoMonsterEvent`))))
    (:`then_1`
      (`TimelineComponent.SetPlayRate` (`self.InitiateSonarCountdown`) (/ 1.0 (- (`self.MonsterEventMinutes`) 1.0)))
      (`Timeline|InitiateSonarCountdown` :!via `PlayFromStart`
        (:`Finished`
          (`self.InitiateSonar`))))))

(event `DoMonsterEvent`
  ;[1 1 1] MONSTER EVENTS
  ;;[1 1 1] Select PseudoRandom Event
  (`|MultiGate` true true
    (:`Out 0`
      (`self.MonsterEventLights`))
    (:`Out 1`
      (`self.MonsterEventHorn`))
    (:`Out 2`
      (`self.MonsterEventSilence`))))

(event `MonsterEventLights`
  ;[1 1 1] MONSTER EVENTS
  ;;[1 1 1] Monster Event |  Lights
  (`/Game/Dynamic/Blueprints/BP_EventManager.ED_StartLightsEvent` (`self.EventManager`))
  (`KismetSystemLibrary.PrintString` "MONSTER EVENT | LUCES")
  (`TimelineComponent.SetPlayRate` (`self.LightsEventCountdown`) (/ 1.0 (`self.EventCountdownSeconds`)))
  (`Timeline|LightsEventCountdown` :!via `PlayFromStart`
    (:`Finished`
      (`self.RestartEventTimer` :!label _label))))

(event `MonsterEventHorn`
  ;[1 1 1] MONSTER EVENTS
  ;;[1 1 1] Monster Event |  Horn
  (`KismetSystemLibrary.PrintString` "MONSTER EVENT | BOCINA")
  (`TimelineComponent.SetPlayRate` (`self.HornEventCountdown`) (/ 1.0 (`self.EventCountdownSeconds`)))
  (`Timeline|HornEventCountdown` :!via `PlayFromStart`
    (:`Finished`
      (`self.RestartEventTimer` :!label _label_2))))

(event `StopLightsEvent`
  ;[1 1 1] MONSTER EVENTS
  ;;[1 1 1] Monster Event |  Lights
  (goto _label))

(event `StopHornEvent`
  ;[1 1 1] MONSTER EVENTS
  ;;[1 1 1] Monster Event |  Horn
  (goto _label_2))

(event `MonsterEventSilence`
  ;[1 1 1] MONSTER EVENTS
  ;;[1 1 1] Monster Event |  Silence
  (`KismetSystemLibrary.PrintString` "MONSTER EVENT | SILENCIO")
  (`TimelineComponent.SetPlayRate` (`self.SilenceEventCountdown`) (/ 1.0 (`self.EventCountdownSeconds`)))
  (`Timeline|SilenceEventCountdown` :!via `PlayFromStart`
    (:`Finished`
      (`self.RestartEventTimer` :!label _label_3))))

(event `StopSilenceEvent`
  ;[1 1 1] MONSTER EVENTS
  ;;[1 1 1] Monster Event |  Silence
  (goto _label_3))

(fn `UserConstructionScript`)