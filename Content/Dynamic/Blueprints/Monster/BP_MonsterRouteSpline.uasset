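; Monster route actor that moves a referenced Actor along a far or close spline during monster events.
; On BeginPlay it finds BP_EventManager and binds to its select, start and end monster-event dispatchers.
; Speed-scaled timelines lerp distance along each spline, setting location and tangent-facing rotation.
; The far run hides the Actor when finished; the close run interrupts it and unhides the Actor, which construction places at the close spline's start.
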(event `self.ReceiveBeginPlay`
  ;[1 1 1] Begin play
  (bind _returnvalue (`GameplayStatics.GetActorOfClass` "/Game/Dynamic/Blueprints/BP_EventManager.BP_EventManager_C"))
  (bind _output_get (set `self.EventManager` _returnvalue))
  (add `/Game/Dynamic/Blueprints/BP_EventManager.ED_SelectMonsterEvent` _output_get (`|CreateDelegate` :!event `PlayFarRangeTimeline`))
  (add `/Game/Dynamic/Blueprints/BP_EventManager.ED_StartMonsterEvent` _output_get (`|CreateDelegate` :!event `PlayCloseRangeTimeline`))
  (add `/Game/Dynamic/Blueprints/BP_EventManager.ED_MonsterEventEnd` _output_get (`|CreateDelegate` :!event `StopCloseTimeline`)))

(event `PlayCloseRangeTimeline`
  (bind _closespline (`self.CloseSpline`))
  (bind _actor (`self.actor`))
  ;[1 0 0] Close
  (`KismetSystemLibrary.PrintString` "CLOSE RANGE")
  (`TimelineComponent.Stop` (`self.FarMovementTimeline`))
  (`self.SetActorHiddenInGame` (`self.actor`) false)
  (`TimelineComponent.SetPlayRate` (`self.CloseMovementTimeline`) (/ 1.0 (`self.CloseRangeSpeed`)))
  (bind (_direction _newtrack_0) (`Timeline|CloseMovementTimeline` :!via `PlayFromStart`)
    (:`Update`
      (bind _returnvalue (`KismetMathLibrary.Lerp` 0.0 (`SplineComponent.GetDistanceAlongSplineAtSplinePoint` _closespline (- (`SplineComponent.GetNumberOfSplinePoints` _closespline) 1)) _newtrack_0))
      (`self.K2_SetActorLocation` _actor (`SplineComponent.GetLocationAtDistanceAlongSpline` _closespline _returnvalue "World") false false)
      (`self.K2_SetActorRotation` _actor (`KismetMathLibrary.Conv_VectorToRotator` (`SplineComponent.GetTangentAtDistanceAlongSpline` (`self.CloseSpline`) _returnvalue "World")) false))))

(event `PlayFarRangeTimeline`
  (bind _farspline (`self.FarSpline`))
  (bind _actor (`self.actor`))
  ;[0.0488 1 0] FAR
  (`KismetSystemLibrary.PrintString` "FAR RANGE")
  (`TimelineComponent.SetPlayRate` (`self.FarMovementTimeline`) (/ 1.0 (`self.FarRangeSpeed`)))
  (bind (_direction _newtrack_0) (`Timeline|FarMovementTimeline` :!via `PlayFromStart`)
    (:`Update`
      (bind _returnvalue (`KismetMathLibrary.Lerp` 0.0 (`SplineComponent.GetDistanceAlongSplineAtSplinePoint` _farspline (- (`SplineComponent.GetNumberOfSplinePoints` _farspline) 1)) _newtrack_0))
      (`self.K2_SetActorLocation` _actor (`SplineComponent.GetLocationAtDistanceAlongSpline` _farspline _returnvalue "World") false false)
      (`self.K2_SetActorRotation` _actor (`KismetMathLibrary.Conv_VectorToRotator` (`SplineComponent.GetTangentAtDistanceAlongSpline` (`self.FarSpline`) _returnvalue "World")) false))
    (:`Finished`
      (`self.SetActorHiddenInGame` (`self.actor`) true))))

(event `StopCloseTimeline`
  ;[1 0 0] Close
  (`TimelineComponent.Stop` (`self.CloseMovementTimeline`)))

(fn `UserConstructionScript`
  (`self.K2_SetActorLocation` (`self.actor`) (`SplineComponent.GetLocationAtSplinePoint` (`self.CloseSpline`) 0 "World") false false))