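; BP_Monster is a monster actor that picks a random monster event and shows a matching shape.
; On BeginPlay it finds BP_EventManager and binds to its select-monster event dispatcher.
; OnSelectedMonsterEvent uses a random, looping MultiGate to set SelectedMonsterEvent to one of three enum values, swap MonsterMesh to a cube, sphere or cone, and unhide the actor.
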(event `self.ReceiveBeginPlay`
  (bind _returnvalue (`GameplayStatics.GetActorOfClass` "/Game/Dynamic/Blueprints/BP_EventManager.BP_EventManager_C"))
  (bind _output_get (set `self.EventManager` _returnvalue))
  (add `/Game/Dynamic/Blueprints/BP_EventManager.ED_SelectMonsterEvent` _output_get (`|CreateDelegate` :!event `OnSelectedMonsterEvent`)))

(event `OnSelectedMonsterEvent`
  (bind _monstermesh (`self.MonsterMesh`))
  ;[1 1 1] Asegura que se ha seleccionado el evento aleatorio correspondiente
  (`|MultiGate` true true
    (:`Out 0`
      (set `self.SelectedMonsterEvent` "NewEnumerator0")
      (`StaticMeshComponent.SetStaticMesh` _monstermesh "/Engine/BasicShapes/Cube.Cube"))
    (:`Out 1`
      (set `self.SelectedMonsterEvent` "NewEnumerator1")
      (`StaticMeshComponent.SetStaticMesh` _monstermesh "/Engine/BasicShapes/Sphere.Sphere"))
    (:`Out 2`
      (set `self.SelectedMonsterEvent` "NewEnumerator2")
      (`StaticMeshComponent.SetStaticMesh` _monstermesh "/Engine/BasicShapes/Cone.Cone")))
  (`self.SetActorHiddenInGame` false))

(fn `UserConstructionScript`)