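; BP_EventManager handles the end of a game, reacting to win and lose events and returning to the lobby level.
; BeginPlay binds both events and caches the level's LevelSequenceActor, which the FadeToBlack macro uses to play a fade sequence.
; Both outcomes record HasSurvived in GI_GameData.
; A win loads L_Lobby after the fade, while a loss plays a sound alongside the fade and loads after the sound's duration.
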(event `self.ReceiveBeginPlay`
  (add `self.ED_WinGame` (`|CreateDelegate` :!event `WinGame`))
  (add `self.ED_LoseGame` (`|CreateDelegate` :!event `LoseGame`))
  (bind _returnvalue (`GameplayStatics.GetActorOfClass` "/Script/LevelSequence.LevelSequenceActor"))
  (set `self.LevelSequence` _returnvalue))

(event `WinGame`
  (bind _asgi_game_data (cast `/Game/Dynamic/Blueprints/GI_GameData` (`GameplayStatics.GetGameInstance`)))
  (set `/Game/Dynamic/Blueprints/GI_GameData.hasSurvived` true _asgi_game_data)
  (`self.FadeToBlack`
    (:`Completed`
      (`GameplayStatics.OpenLevelBySoftObjectPtr` "/Game/Dynamic/Maps/L_Lobby.L_Lobby" :!label _label))))

(event `LoseGame`
  (bind _endgameonlosesound (`self.EndGameOnLoseSound`))
  (bind _asgi_game_data (cast `/Game/Dynamic/Blueprints/GI_GameData` (`GameplayStatics.GetGameInstance`)))
  (set `/Game/Dynamic/Blueprints/GI_GameData.hasSurvived` false _asgi_game_data)
  (`GameplayStatics.PlaySound2D` _endgameonlosesound 1.0 1.0 0.0 null null)
  (`|ExecutionSequence`
    (:`then_0`
      (`self.FadeToBlack`))
    (:`then_1`
      (`KismetSystemLibrary.Delay` (`SoundBase.Duration` _endgameonlosesound))
      (goto _label))))

(fn `UserConstructionScript`)