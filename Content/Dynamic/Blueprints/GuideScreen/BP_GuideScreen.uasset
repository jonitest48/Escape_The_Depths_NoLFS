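; BP_GuideScreen is a screen that cycles through an image carousel in an endless loop.
; On BeginPlay it puts a dynamic instance of MI_ContenidoPantalla on the ContenidoPantalla component and shows the first ImageCarrousel texture.
; A fast looping timer starts each pass, pausing itself while a delayed for-each loop swaps the "Contenido" texture every BetweenImageDelay, then resuming to restart the cycle.
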(event `self.ReceiveBeginPlay`
  (bind _returnvalue (`KismetMaterialLibrary.CreateDynamicMaterialInstance` "/Game/Dynamic/Materials/MI/MI_ContenidoPantalla.MI_ContenidoPantalla"))
  (bind _output_get (set `self.DynamicMaterial` _returnvalue))
  (`PrimitiveComponent.SetMaterial` (`self.ContenidoPantalla`) 0 _output_get)
  (`MaterialInstanceDynamic.SetTextureParameterValue` (`self.DynamicMaterial`) "Contenido" (`|GetArrayItem` (`self.ImageCarrousel`)))
  (bind _returnvalue_2 (`KismetSystemLibrary.K2_SetTimerDelegate` (delegate `StartImageCarrousel`) 0.01 true))
  (set `self.EventTimer` _returnvalue_2))

(event `StartImageCarrousel`
  (`KismetSystemLibrary.K2_PauseTimerHandle` (`self.EventTimer`))
  (bind _array_element (`/Game/Dynamic/Blueprints/BP_MacroUtils.For Each Loop With Delay` (`self.ImageCarrousel`) (`self.BetweenImageDelay`))
    (:`Loop Body`
      (`MaterialInstanceDynamic.SetTextureParameterValue` (`self.DynamicMaterial`) "Contenido" _array_element))
    (:`Completed`
      (`KismetSystemLibrary.K2_UnPauseTimerHandle` (`self.EventTimer`)))))

(fn `UserConstructionScript`)