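; Controller for the submarine's timed monster events (Lights, Horn, Silence), looping once power turns on.
; BP_EventManager dispatchers link it to the level; a countdown starts the event selected on BP_Monster, while another triggers selection and accelerating sonar pings.
; Lights and Horn damage the submarine unless stopped before timeout, whereas stopping Silence early causes damage.
; Each outcome hides the monster, silences the sonar and restarts the cycle.
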(event `self.ReceiveBeginPlay`
  ;[1 1 1] On Begin | Enable Monster Event Timer
  (set `self.BetweenEventSeconds` (* 60.0 (`self.BetweenEventMinutes`)))
  (set `self.EventCountdownSeconds` (* 60.0 (`self.EventCountdownMinutes`)))
  (bind _returnvalue (`GameplayStatics.GetActorOfClass` "/Game/Dynamic/Blueprints/BP_EventManager.BP_EventManager_C"))
  (set `self.EventManager` _returnvalue)
  (bind _returnvalue_2 (`GameplayStatics.GetActorOfClass` "/Game/Dynamic/Blueprints/Monster/BP_Monster.BP_Monster_C"))
  (set `self.Monster` _returnvalue_2)
  (`self.Bind Events to Event Manager` (`self.EventManager`)))

(event `InitiateSonar`
  (bind _sonarsound (`self.SonarSound`))
  (bind _returnvalue (`TimelineComponent.GetPlayRate` _sonarsound))
  ;[1 1 1] SONAR
  (`TimelineComponent.SetPlayRate` (`self.SonarSound`) 1.0)
  (`Timeline|SonarSound` :!via `PlayFromStart`
    (:`SonarSoundTrack`
      (if (not (>= _returnvalue 4.0))
        (`TimelineComponent.SetPlayRate` _sonarsound (+ _returnvalue 0.08)))
      (`GameplayStatics.PlaySound2D` "/Game/Dynamic/Audio/Sonar/submarine-sonar-38243_Edited.submarine-sonar-38243_Edited" 1.0 1.0 0.0 null null))))

(event `BeginMonsterEventsCounter`
  ;[1 1 1] START MONSTER EVENTS ON POWER ON (LOOP)
  (`|ExecutionSequence`
    (:`then_0`
      (`TimelineComponent.SetPlayRate` (`self.InitiateMonsterEventCountdown`) (/ 1.0 (`self.BetweenEventMinutes`)))
      (`Timeline|InitiateMonsterEventCountdown` :!via `PlayFromStart`
        (:`Finished`
          (`self.DoMonsterEvent`))))
    (:`then_1`
      (`TimelineComponent.SetPlayRate` (`self.InitiateSonarCountdown`) (/ 1.0 (- (`self.EventCountdownMinutes`) 60.0)))
      (`Timeline|InitiateSonarCountdown` :!via `PlayFromStart`
        (:`Finished`
          (`self.InitiateSonar`)
          (`/Game/Dynamic/Blueprints/BP_EventManager.ED_SelectMonsterEvent` (`self.EventManager`)))))))

(event `DoMonsterEvent`
  (bind _eventmanager (`self.EventManager`))
  ;[1 1 1] MONSTER EVENTS
  ;;[1 1 1] Select PseudoRandom Event
  (switch `/Game/Dynamic/Blueprints/MonsterEvents/E_MonsterEvents` (`/Game/Dynamic/Blueprints/Monster/BP_Monster.SelectedMonsterEvent` (`self.Monster`))
    (:`NewEnumerator0`
      ;;;[1 1 1] Llamada con dispatcher para activar en el nivel todo lo necesario para el evento además del contador y condiciones situado en este mismo BP
      (`/Game/Dynamic/Blueprints/BP_EventManager.ED_StartLightsEvent` _eventmanager))
    (:`NewEnumerator1`
      (`/Game/Dynamic/Blueprints/BP_EventManager.ED_StartHornEvent` _eventmanager))
    (:`NewEnumerator2`
      (`/Game/Dynamic/Blueprints/BP_EventManager.ED_StartSilenceEvent` _eventmanager))))

(event `StartLightsEvent`
  ;[1 1 1] MONSTER EVENTS
  ;;[1 1 1] Monster Event |  Lights
  (`KismetSystemLibrary.PrintString` "MONSTER EVENT | LUCES")
  (`TimelineComponent.SetPlayRate` (`self.LightsEventCountdown`) (/ 1.0 (`self.EventCountdownSeconds`)))
  (`Timeline|LightsEventCountdown` :!via `PlayFromStart` :!label _label
    (:`Finished`
      (`/Game/Dynamic/Blueprints/BP_EventManager.ED_DamageSubmarine` (`self.EventManager`))
      (`KismetSystemLibrary.PrintString` "EVENTO FALLIDO" true true (struct :`R` 1.0 :`B` 0.116351 :`A` 1.0))
      (`self.RestartEventTimer` :!label _label_2))))

(event `StartHornEvent`
  ;[1 1 1] MONSTER EVENTS
  ;;[1 1 1] Monster Event |  Horn
  (`KismetSystemLibrary.PrintString` "MONSTER EVENT | BOCINA")
  (`TimelineComponent.SetPlayRate` (`self.HornEventCountdown`) (/ 1.0 (`self.EventCountdownSeconds`)))
  (`Timeline|HornEventCountdown` :`NewTime` 1.0 :!via `PlayFromStart` :!label _label_3
    (:`Finished`
      (`/Game/Dynamic/Blueprints/BP_EventManager.ED_DamageSubmarine` (`self.EventManager`))
      (`KismetSystemLibrary.PrintString` "EVENTO FALLIDO" true true (struct :`R` 1.0 :`B` 0.116351 :`A` 1.0))
      (`self.RestartEventTimer` :!label _label_4))))

(event `StopLightsEvent`
  ;[1 1 1] MONSTER EVENTS
  ;;[1 1 1] Monster Event |  Lights
  (if (`|EnumEquality` (`/Game/Dynamic/Blueprints/Monster/BP_Monster.SelectedMonsterEvent` (`self.Monster`)) "NewEnumerator0")
    (`|ExecutionSequence`
      (:`then_0`
        (goto _label :!via `Stop`))
      (:`then_1`
        (`KismetSystemLibrary.PrintString` "EVENTO SUPERADO" true true (struct :`R` 0.057249 :`G` 1.0 :`A` 1.0))
        (goto _label_2)))))

(event `StopHornEvent`
  ;[1 1 1] MONSTER EVENTS
  ;;[1 1 1] Monster Event |  Horn
  (if (`|EnumEquality` (`/Game/Dynamic/Blueprints/Monster/BP_Monster.SelectedMonsterEvent` (`self.Monster`)) "NewEnumerator1")
    (`|ExecutionSequence`
      (:`then_0`
        (goto _label_3 :!via `Stop`))
      (:`then_1`
        (`KismetSystemLibrary.PrintString` "EVENTO SUPERADO" true true (struct :`R` 0.134947 :`G` 1.0 :`A` 1.0))
        (goto _label_4)))))

(event `StartSilenceEvent`
  ;[1 1 1] MONSTER EVENTS
  ;;[1 1 1] Monster Event |  Silence
  (`KismetSystemLibrary.PrintString` "MONSTER EVENT | SILENCIO")
  (`TimelineComponent.SetPlayRate` (`self.SilenceEventCountdown`) (/ 1.0 (`self.EventCountdownSeconds`)))
  (`Timeline|SilenceEventCountdown` :!via `PlayFromStart` :!label _label_5
    (:`Finished`
      (`KismetSystemLibrary.PrintString` "EVENTO SUPERADO" true true (struct :`R` 0.143117 :`G` 1.0 :`A` 1.0))
      (`self.RestartEventTimer` :!label _label_6))))

(event `StopSilenceEvent`
  ;[1 1 1] MONSTER EVENTS
  ;;[1 1 1] Monster Event |  Silence
  (`|ExecutionSequence`
    (:`then_0`
      (goto _label_5 :!via `Stop`))
    (:`then_1`
      (`/Game/Dynamic/Blueprints/BP_EventManager.ED_DamageSubmarine` (`self.EventManager`))
      (`KismetSystemLibrary.PrintString` "EVENTO FALLIDO" true true (struct :`R` 1.0 :`B` 0.116351 :`A` 1.0))
      (goto _label_6))))

(fn `Bind Events to Event Manager`
  (params (EventManager :type "/Game/Dynamic/Blueprints/BP_EventManager Object Reference"))
  (bind _eventmanager (`self.EventManager`))
  (add `/Game/Dynamic/Blueprints/BP_EventManager.ED_TurnPowerOn` EventManager (`|CreateDelegate` :!event `BeginMonsterEventsCounter`))
  (`|ExecutionSequence`
    (:`then_0`
      (add `/Game/Dynamic/Blueprints/BP_EventManager.ED_StartLightsEvent` _eventmanager (`|CreateDelegate` :!event `StartLightsEvent`))
      (add `/Game/Dynamic/Blueprints/BP_EventManager.ED_StartHornEvent` _eventmanager (`|CreateDelegate` :!event `StartHornEvent`))
      (add `/Game/Dynamic/Blueprints/BP_EventManager.ED_StartSilenceEvent` _eventmanager (`|CreateDelegate` :!event `StartSilenceEvent`)))
    (:`then_1`
      (add `/Game/Dynamic/Blueprints/BP_EventManager.ED_StopLightsEvent` _eventmanager (`|CreateDelegate` :!event `StopLightsEvent`))
      (add `/Game/Dynamic/Blueprints/BP_EventManager.ED_StopHornEvent` _eventmanager (`|CreateDelegate` :!event `StopHornEvent`))
      (add `/Game/Dynamic/Blueprints/BP_EventManager.ED_StopSilenceEvent` _eventmanager (`|CreateDelegate` :!event `StopSilenceEvent`)))))

(fn `UserConstructionScript`)