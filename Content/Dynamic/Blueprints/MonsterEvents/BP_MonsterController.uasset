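; BP_MonsterController schedules periodic monster events, with lights, horn and silence variants that are currently only debug-print stubs.
; BeginPlay starts a looping timer from a minutes setting and binds the event manager's power-on dispatcher to unpause it.
; DoMonsterEvent picks a variant through a random, looping MultiGate.
; Lights pauses the timer while horn and silence unpause it, and DoMonsterEvent also has an unpause after the gate.
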(event `self.ReceiveBeginPlay`
  ;[1 1 1] On Begin | Enable Monster Event Timer
  (set `self.TimeBetweenMonsterEvent` (* 60.0 (`self.MonsterEventMinutes`)))
  (bind _returnvalue (`GameplayStatics.GetActorOfClass` "/Game/Dynamic/Blueprints/BP_EventManager.BP_EventManager_C"))
  (bind _output_get (set `self.EventManager` _returnvalue))
  (add `/Game/Dynamic/Blueprints/BP_EventManager.ED_TurnPowerOn` _output_get (delegate `StartMonsterEventTimer`))
  (bind _returnvalue_2 (`KismetSystemLibrary.K2_SetTimerDelegate` (`|CreateDelegate` :!event `DoMonsterEvent`) (`self.TimeBetweenMonsterEvent`) true))
  (bind _output_get_2 (set `self.MonsterTimer` _returnvalue_2)))

(event `StartMonsterEventTimer`
  ;[1 1 1] On Begin | Enable Monster Event Timer
  (`KismetSystemLibrary.K2_UnPauseTimerHandle` (`self.MonsterTimer`)))

(event `DoMonsterEvent`
  ;[1 1 1] MONSTER EVENTS
  ;;[1 1 1] Select PseudoRandom Event
  (`|MultiGate` true true
    (:`Out 0`
      (`self.MonsterEventLights`))
    (:`Out 1`
      (`self.MonsterEventHorn`))
    (:`Out 2`
      (`self.MonsterEventSilence`)))
  (`KismetSystemLibrary.K2_UnPauseTimerHandle` (`self.MonsterTimer`)))

(event `MonsterEventLights`
  ;[1 1 1] MONSTER EVENTS
  ;;[1 1 1] Monster Event |  Lights
  (`KismetSystemLibrary.K2_PauseTimerHandle` (`self.MonsterTimer`))
  (`KismetSystemLibrary.PrintString` "MONSTER EVENT | LUCES"))

(event `MonsterEventHorn`
  ;[1 1 1] MONSTER EVENTS
  ;;[1 1 1] Monster Event |  Horn
  (`KismetSystemLibrary.PrintString` "MONSTER EVENT | BOCINA")
  (`KismetSystemLibrary.K2_UnPauseTimerHandle` (`self.MonsterTimer`)))

(event `MonsterEventSilence`
  ;[1 1 1] MONSTER EVENTS
  ;;[1 1 1] Monster Event |  Silence
  (`KismetSystemLibrary.PrintString` "MONSTER EVENT | SILENCIO")
  (`KismetSystemLibrary.K2_UnPauseTimerHandle` (`self.MonsterTimer`)))

(fn `UserConstructionScript`)