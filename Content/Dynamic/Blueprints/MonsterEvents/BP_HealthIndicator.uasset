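; BP_HealthIndicator tracks submarine health and shows it as the color of an indicator cube.
; On BeginPlay it binds to the BP_EventManager submarine damage dispatcher, then turns green after a short delay.
; Each hit plays a metal impact sound, decrements health and recolors the cube through a material parameter.
; At zero health it darkens the cube and calls the manager's lose-game dispatcher.
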(event `self.ReceiveBeginPlay`
  (bind _returnvalue (`GameplayStatics.GetActorOfClass` "/Game/Dynamic/Blueprints/BP_EventManager.BP_EventManager_C"))
  (`/Engine/EditorBlueprintResources/StandardMacros.IsValid` _returnvalue
    (:`Is Valid`
      (set `self.EventManager` _returnvalue)
      (add `/Game/Dynamic/Blueprints/BP_EventManager.ED_DamageSubmarine` (`self.EventManager`) (`|CreateDelegate` :!event `Receive Damage`))
      (`KismetSystemLibrary.Delay` 2.0)
      (`self.ChangeIndicatorColor` (struct :`R` 0.020661 :`G` 0.510417 :`B` 0.038107 :`A` 1.0)))))

(event `Receive Damage`
  (`GameplayStatics.PlaySound2D` "/Game/Dynamic/Audio/metal-impact.metal-impact" 1.0 1.0 0.0 null null)
  (bind _result (`/Engine/EditorBlueprintResources/StandardMacros.DecrementInt` (`self.SubmarineHealth`))
    (:`  `
      (switch `int` _result
        (:`0`
          (`self.ChangeIndicatorColor` (struct :`R` 0.020833 :`G` 0.020833 :`B` 0.020833 :`A` 1.0))
          (`/Game/Dynamic/Blueprints/BP_EventManager.ED_LoseGame` (`self.EventManager`)))
        (:`1`
          (`self.ChangeIndicatorColor` (struct :`R` 0.453125 :`B` 0.035244 :`A` 1.0)))
        (:`2`
          (`self.ChangeIndicatorColor` (struct :`R` 0.71875 :`G` 0.241056 :`B` 0.022662 :`A` 1.0)))))))

(fn `ChangeIndicatorColor`
  (params (HealthIndicatorColor :type "LinearColor Structure"))
  (bind _output_get (set `self.HealthIndicatorColor` HealthIndicatorColor))
  (`MeshComponent.SetVectorParameterValueOnMaterials` (`self.IndicatorCube`) "Color" (`KismetMathLibrary.Conv_LinearColorToVector` _output_get)))

(fn `UserConstructionScript`)