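; Pressable button for the lights monster event that switches emergency mode on and off through the EventManager.
; Pressing runs the parent logic behind a re-entry gate and emits a sound alert; toggling only takes effect while powered, and restored power reapplies the button's state.
; Emergency mode starts a timeline countdown, rate-scaled to the event duration, which on finishing stops the lights event and releases the button.
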(event `self.ReceiveBeginPlay`
  (bind _eventmanager (`self.EventManager`))
  ;[1 1 1] Begin Play
  (`parent.ReceiveBeginPlay`)
  (add `/Game/Dynamic/Blueprints/BP_EventManager.ED_StartLightsEvent` _eventmanager (delegate `ActivateEmergencyLight`))
  (add `/Game/Dynamic/Blueprints/BP_EventManager.ED_TurnPowerOn` _eventmanager (`|CreateDelegate` :!event `TurnPowerOn`)))

(event `ActivateEmergencyLight`
  ;[1 1 1] Begin Play
  (set `self.isEventActive` true))

(event `/Game/Dynamic/Blueprints/Interfaces/BPI_Button.Press`
  ;[1 1 1] EventPress
  (`/Engine/EditorBlueprintResources/StandardMacros.Gate` false :!label _label
    (:`Exit`
      (`|ExecutionSequence`
        (:`then_0`
          (goto _label :!via `Close`))
        (:`then_1`
          (`parent.Press`)
          (`/Game/Dynamic/Blueprints/MonsterEvents/3_Silence/BP_SilenceEventFunctions.SoundAlertAtLocation` "/Game/Dynamic/Audio/Button.Button" (`SceneComponent.K2_GetComponentLocation` (`self.DefaultSceneRoot`)) (`self.EventManager`))
          (goto _label :!via `Open`))))))

(event `self.OnPressAction`
  ;[1 1 1] Interaccion boton
  (if (`self.isPowered`)
    (`/Game/Dynamic/Blueprints/BP_EventManager.ED_EmergencyModeOn` (`self.EventManager`))
    (`self.StartEventCountdown`)))

(event `/Game/Dynamic/Blueprints/Interfaces/BPI_Button.OnUnpressAction`
  ;[1 1 1] Interaccion boton
  (if (`self.isPowered`)
    (`/Game/Dynamic/Blueprints/BP_EventManager.ED_EmergencyModeOff` (`self.EventManager`))
    (`TimelineComponent.Stop` (`self.EmergencyModeCountdown`))))

(event `/Game/Dynamic/Blueprints/Interfaces/BPI_LightPowered.TurnPowerOn`
  (bind _eventmanager (`self.EventManager`))
  ;[1 1 1] Power On
  (set `self.isPowered` true)
  (if (`self.isButtonPressed`)
    (`/Game/Dynamic/Blueprints/BP_EventManager.ED_EmergencyModeOn` _eventmanager)
    (`self.StartEventCountdown`)
    (else
      (`/Game/Dynamic/Blueprints/BP_EventManager.ED_EmergencyModeOff` _eventmanager)
      (`TimelineComponent.Stop` (`self.EmergencyModeCountdown`)))))

(event `/Game/Dynamic/Blueprints/Interfaces/BPI_LightPowered.TurnPowerOff`
  ;[1 1 1] Power On
  (set `self.isPowered` false))

(event `StartEventCountdown`
  ;[1 1 1] Event Countdown
  (`TimelineComponent.SetPlayRate` (`self.EmergencyModeCountdown`) (/ 1.0 (`self.Event Completion Seconds`)))
  (`Timeline|EmergencyModeCountdown` :!via `PlayFromStart`
    (:`Finished`
      (`/Game/Dynamic/Blueprints/BP_EventManager.ED_StopLightsEvent` (`self.EventManager`))
      (if (`self.isEventActive`)
        (set `self.isEventActive` false))
      (`self.Unpress`))))

(fn `getIsPowered`
  (returns (isPowered :type Boolean))
  (return (`self.isPowered`)))

(fn `UserConstructionScript`
  (`parent.UserConstructionScript`))