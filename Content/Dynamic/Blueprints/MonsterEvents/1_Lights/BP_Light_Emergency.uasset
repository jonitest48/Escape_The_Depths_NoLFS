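; Emergency light Blueprint whose point light is visible only while emergency mode is active.
; On BeginPlay it finds BP_EventManager and binds to its emergency mode on and off dispatchers, which set IsEmergencyMode and the light's visibility.
; The construction script applies the same state from IsEmergencyMode, and GetIsPowered reports that flag as the light's powered state.
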(event `self.ReceiveBeginPlay`
  (bind _eventmanager (`self.EventManager`))
  ;[1 1 1] EventManager Bind
  (bind _returnvalue (`GameplayStatics.GetActorOfClass` "/Game/Dynamic/Blueprints/BP_EventManager.BP_EventManager_C"))
  (set `self.EventManager` _returnvalue)
  (add `/Game/Dynamic/Blueprints/BP_EventManager.ED_EmergencyModeOn` _eventmanager (`|CreateDelegate` :!event `EmergencyModeOn`))
  (add `/Game/Dynamic/Blueprints/BP_EventManager.ED_EmergencyModeOff` _eventmanager (`|CreateDelegate` :!event `EmergencyModeOff`)))

(event `EmergencyModeOn`
  (bind _output_get (set `self.Is EmergencyMode` true))
  (`SceneComponent.SetVisibility` (`self.PointLight`) _output_get false))

(event `EmergencyModeOff`
  (bind _output_get (set `self.Is EmergencyMode` false))
  (`SceneComponent.SetVisibility` (`self.PointLight`) _output_get false))

(fn `getIsPowered`
  (returns (isPowered :type Boolean))
  (return (`self.Is EmergencyMode`)))

(fn `UserConstructionScript`
  (if (`self.Is EmergencyMode`)
    (`self.EmergencyModeOn`)
    (else
      (`self.EmergencyModeOff`))))